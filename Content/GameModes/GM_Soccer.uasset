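; Game mode for a soccer level that runs a countdown timer and handles losing and level completion.
; A looping one-second timer decrements the time and updates the timer widget, showing the lose widget when it expires.
; Tick polls the player character's remaining balls and opens the LoseMenu level when none are left.
; ShowNextLevel displays the next-level win menu with UI-only input and a visible cursor.
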(event EventBeginPlay
  (Utilities|Time|SetTimerbyFunctionName 0 "CountDown" 1.0 true)
  (bind _returnvalue (UserInterface|CreateWidget "/Game/UI/WB_Timer.WB_Timer_C"))
  (bind _output_get (Variables|Default|SetTimerWidget _returnvalue))
  (UserInterface|Viewport|AddtoViewport _output_get 0)
  (Input|SetInputModeGameOnly (Game|GetPlayerController 0) false))

(event EventTick
  (params (DeltaSeconds :type Float%20%28single-precision%29))
  (bind _asbp_player_character (Utilities|Casting|CastToBP_PlayerCharacter (Game|GetPlayerCharacter 0)))
  (bind _returnvalue (Class|PlayerCharacter|GetBallsLeft _asbp_player_character))
  (if (<= _returnvalue 0)
    (Game|OpenLevel(byName) "LoseMenu")))

(fn ConstructionScript)

(fn CountDown
  (bind _returnvalue (Game|GetPlayerController 0))
  (Variables|Default|SetTotalTime (- (Variables|Default|GetTotalTime) 1.0))
  (Default|UpdateTimerText (Variables|Default|GetTimerWidget) (Utilities|Text|FormatText "{0}:{1}" (Math|Conversions|ToFloat(Integer) (Class|KismetMathLibrary|ToInt64(Float) (/ (Variables|Default|GetTotalTime) 6e+01))) (Math|Float|%(Float) (Variables|Default|GetTotalTime) 6e+01)))
  (if (<= (Variables|Default|GetTotalTime) 0.0)
    (Utilities|Time|ClearTimerbyFunctionName 0 "CountDown")
    (bind _returnvalue_2 (UserInterface|CreateWidget "/Game/UI/WB_LoseMenu.WB_LoseMenu_C"))
    (UserInterface|Viewport|AddtoViewport _returnvalue_2 0)
    (Input|SetInputModeUIOnly _returnvalue 0 "DoNotLock" false)
    (Variables|/Script/Engine.PlayerController|SetbShowMouseCursor _returnvalue true)))

(fn ShowNextLevel
  (bind _returnvalue (Game|GetPlayerController 0))
  (bind _returnvalue_2 (UserInterface|CreateWidget "/Game/UI/WB_NextLevelWinMenu.WB_NextLevelWinMenu_C"))
  (UserInterface|Viewport|AddtoViewport _returnvalue_2 0)
  (Input|SetInputModeUIOnly _returnvalue 0 "DoNotLock" false)
  (Variables|/Script/Engine.PlayerController|SetbShowMouseCursor _returnvalue true))