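; BP_MovingObstacles is a moving electric hazard that damages the player's BP_ControllableCharacter when it enters the obstacle's capsule.
; The construction script sets an InterpToMovement path from the origin to a relative MoveToPoint, with Speed used as the travel duration.
; It also positions a sphere and sizes the capsule from Length, while LightningLength scales the Niagara zap effect.
; Overlap hits are gated by CanDamage, which a half-second timer resets.
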(event OnComponentBeginOverlap(Capsule)
  (params (OverlappedComponent :type Primitive%20Component%20Object%20Reference) (OtherActor :type Actor%20Object%20Reference) (OtherComp :type Primitive%20Component%20Object%20Reference) (OtherBodyIndex :type Integer) (bFromSweep :type Boolean) (SweepResult :type Hit%20Result%20Structure%20%28by%20ref%29))
  (if (== OtherActor (Game|Player|GetPlayerPawn 0))
    (if (Variables|Default|GetCanDamage)
      (Class|ControllableCharacter|TakeDamage (Variables|Default|GetAs%20BP%20Controllable%20Character))
      (Variables|Default|SetCanDamage false)
      (Utilities|Time|SetTimerbyFunctionName 0 "Damage CD" 0.5))))

(event EventBeginPlay
  (bind _asbp_controllable_character (Utilities|Casting|CastToBP_ControllableCharacter (Game|Player|GetPlayerPawn 0)))
  (Variables|Default|SetAs%20BP%20Controllable%20Character _asbp_controllable_character))

(event Collision|EventActorBeginOverlap
  (params (OtherActor :type Actor%20Object%20Reference)))

(event EventTick
  (params (DeltaSeconds :type Float%20%28single-precision%29)))

(fn ConstructionScript
  (bind _interptomovement (Variables|Default|GetInterpToMovement))
  (bind _capsule (Variables|Collision|GetCapsule))
  (bind _length (Variables|Default|GetLength))
  (bind _returnvalue (/ _length 2.0))
  (Class|InterptoMovementComponent|AddControlPointPosition _interptomovement "0, 0, 0" true)
  (Class|InterptoMovementComponent|AddControlPointPosition _interptomovement (Variables|Default|GetMoveToPoint) true)
  (Variables|/Script/Engine.InterpToMovementComponent|SetDuration _interptomovement (Variables|Default|GetSpeed))
  (Transformation|SetRelativeLocation (Variables|Default|GetSphere1) (Math|Vector|MakeVector 0.0 0.0 _length) false false)
  (Components|Capsule|SetCapsuleHalfHeight _capsule _returnvalue true)
  (Transformation|SetRelativeLocation _capsule (Math|Vector|MakeVector 0.0 0.0 _returnvalue) false false)
  (Niagara|SetNiagaraVariable(Float) (Variables|Default|GetNS_Zap_Custom) "Lightning Scale Vertical" (Variables|Default|GetLightningLength)))

(fn DamageCD
  (Variables|Default|SetCanDamage true))